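; Enemy Blueprint that tracks hit points and destroys itself when they run out.
; A Damaged event subtracts incoming damage from HP.
; Tick polls HP every frame and, at zero or below, prints a death message and calls Die, which destroys the actor.
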(event EventBeginPlay)

(event Collision|EventActorBeginOverlap
  (params (OtherActor :type Actor%20Object%20Reference)))

(event EventTick
  (params (DeltaSeconds :type Float%20%28single-precision%29))
  (if (<= (Variables|Default|GetHP) 0)
    (Development|PrintString "Enemy Died")
    (CallFunction|Die)))

(event Custom|Damaged
  (params (DamagePoint :type Integer))
  (Variables|Default|SetHP (- (Variables|Default|GetHP) DamagePoint)))

(event Custom|Die
  (Actor|DestroyActor))

(fn ConstructionScript)